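; BP_EnemyBoss is a space shooter boss enemy that sweeps sideways between boundaries, extending a parent enemy class.
; BeginPlay sets its lives and starts it moving along its right vector.
; Overlaps with "Lateral"-tagged actors flip the movement vector: the leftward leg adds negative-X drift and shortens the shot delay, while the rightward leg restores the plain right vector.
; Tick only calls the parent.
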(event `self.ReceiveBeginPlay`
  (`parent.ReceiveBeginPlay`)
  (set `self.Lives` 2)
  (set `self.MovementVector` (`self.GetActorRightVector`))
  (set `self.IsRight` true))

(event `self.ReceiveActorBeginOverlap`
  (params (OtherActor :type "Actor Object Reference"))
  (bind _returnvalue (`self.GetActorRightVector`))
  (`parent.ReceiveActorBeginOverlap` OtherActor)
  (if (`KismetArrayLibrary.Array_Contains` (`Actor.Tags` OtherActor) "Lateral")
    (if (`self.IsRight`)
      (set `self.IsRight` false)
      (set `self.MovementVector` (`KismetMathLibrary.MakeVector` -0.5 (.y (* _returnvalue -1.0)) (.z (* _returnvalue -1.0))))
      (set `self.DelayShoot` (- (`self.DelayShoot`) 0.1))
      (else
        (set `self.IsRight` true)
        (set `self.MovementVector` _returnvalue)))))

(event `self.ReceiveTick`
  (params (DeltaSeconds :type "Float (single-precision)"))
  (`parent.ReceiveTick` DeltaSeconds))

(fn `UserConstructionScript`
  (`parent.UserConstructionScript`))